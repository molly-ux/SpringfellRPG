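; BP_Enemy is an enemy Blueprint that handles taking damage and dying through its AnyDamage event.
; Every hit plays a sound, and while Health is above zero it subtracts damage, spawns a particle effect and plays a hit montage.
; A hit at zero or less Health calls EnemyDeath on the AI_Enemy controller, plays a death montage, activates Niagara and increments the player's EnemiesKilled count.
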(event Game|Damage|EventAnyDamage
  (params (Damage :type Float%20%28single-precision%29) (DamageType :type Damage%20Type%20Object%20Reference) (InstigatedBy :type Controller%20Object%20Reference) (DamageCauser :type Actor%20Object%20Reference))
  (Audio|PlaySound2D "/Game/Audio/VO/SC_EnemyHit.SC_EnemyHit" 0.5 1.0 0.0 0 0 false)
  (if (> (Variables|Default|GetHealth) 0.0)
    (Variables|Default|SetHealth (- (Variables|Default|GetHealth) Damage))
    (Effects|SpawnEmitteratLocation "/Game/FXVarietyPack/Particles/P_ky_hit2.P_ky_hit2" (Transformation|GetActorLocation) "0, 0, 0" "0.200000,0.200000,0.200000")
    (Animation|PlayAnimMontage "/Game/Characters/Enemy/Animations/AM_EnemyHit.AM_EnemyHit" 1.5 "None")
    (else
      (bind _asai_enemy (Utilities|Casting|CastToAI_Enemy (Pawn|GetController)))
      (Default|EnemyDeath _asai_enemy)
      (Animation|PlayAnimMontage "/Game/Characters/Enemy/Animations/AM_EnemyDeathA.AM_EnemyDeathA" 1.0 "None")
      (Components|Activation|Activate (Variables|Default|GetNiagara) false)
      (bind _asbp_third_person_character (Utilities|Casting|CastToBP_ThirdPersonCharacter (Game|GetPlayerCharacter 0)))
      (bind _output_get (Variables|/Game/ThirdPerson/Blueprints/BP_ThirdPersonCharacter.BP_ThirdPersonCharacter_C|SetEnemiesKilled _asbp_third_person_character (+ (Variables|/Game/ThirdPerson/Blueprints/BP_ThirdPersonCharacter.BP_ThirdPersonCharacter_C|GetEnemiesKilled _asbp_third_person_character) 1.0)))
      (Development|PrintString (Utilities|String|ToString(Float) _output_get)))))

(fn ConstructionScript)